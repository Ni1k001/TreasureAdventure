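; Player controller Blueprint that toggles the pause menu when the Pause input is pressed.
; Pausing clears all widgets, pauses the game, disables pawn input and shows W_PauseMenu in Game and UI mode with keyboard focus on its Resume button.
; Unpausing clears all widgets, restores game-only input and pawn control, hides the cursor and creates a fresh PlayerHUD instead of reusing the previous one.
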(event Input|ActionEvents|InputActionPause
  (params (Key :type Key%20Structure))
  (bind _returnvalue (Game|GetPlayerController 0))
  (bind _returnvalue_2 (Game|GetPlayerController 0))
  (:Pressed
    (if (Game|IsGamePaused)
      (Viewport|RemoveAllWidgets)
      (Game|SetGamePaused false)
      (Variables|/Script/Engine.PlayerController|SetbShowMouseCursor _returnvalue_2 false)
      (bind _returnvalue_3 (UserInterface|CreateWidget "/Game/Widgets/PlayerHUD.PlayerHUD_C"))
      (Input|SetInputModeGameOnly _returnvalue_2)
      (Input|EnableInput (Pawn|GetControlledPawn _returnvalue_2) _returnvalue_2)
      (UserInterface|Viewport|AddtoViewport _returnvalue_3 0)
      (else
        (Viewport|RemoveAllWidgets)
        (bind _returnvalue_4 (Game|SetGamePaused true))
        (Variables|/Script/Engine.PlayerController|SetbShowMouseCursor _returnvalue _returnvalue_4)
        (bind _returnvalue_5 (UserInterface|CreateWidget "/Game/Widgets/W_PauseMenu.W_PauseMenu_C"))
        (Input|SetInputModeGameandUI _returnvalue (Variables|/Game/Widgets/UIButton.UIButton_C|GetButton (Variables|/Game/Widgets/W_PauseMenu.W_PauseMenu_C|GetResumeButton _returnvalue_5)) "DoNotLock" true)
        (Input|DisableInput (Pawn|GetControlledPawn _returnvalue) _returnvalue)
        (UserInterface|Viewport|AddtoViewport _returnvalue_5 0)
        (Widget|SetKeyboardFocus (Variables|/Game/Widgets/UIButton.UIButton_C|GetButton (Variables|/Game/Widgets/W_PauseMenu.W_PauseMenu_C|GetResumeButton _returnvalue_5)))))))

(fn ConstructionScript)