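; Game Instance Blueprint that switches the game's top-level UI and relays level streaming changes.
; SetWidget takes a selection, clears all widgets, then creates the matching main menu, level selector, HUD, loading screen or pause menu for player controller 0.
; The new widget is stored as CurrentWidget and added to the viewport, while None only clears the screen.
; The OnLevelStreamingChange event fires OnChange.
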(event EventOnLevelStreamingChange
  (Default|CallOnChange))

(fn SetWidget
  (params (Selection :type WidgetEnum%20Enum :default "ENone"))
  (switch Utilities|FlowControl|Switch|SwitchonWidgetEnum Selection
    (:ENone
      (Viewport|RemoveAllWidgets))
    (:EMainMenuWidget
      (Viewport|RemoveAllWidgets)
      (bind _returnvalue (UserInterface|CreateWidget "/Game/Widgets/W_MainMenu.W_MainMenu_C" (Game|GetPlayerController 0)))
      (bind _output_get (Variables|Default|SetCurrentWidget _returnvalue))
      (UserInterface|Viewport|AddtoViewport _output_get 0))
    (:ELevelLoadingWidget
      (Viewport|RemoveAllWidgets)
      (bind _returnvalue_2 (UserInterface|CreateWidget "/Game/Widgets/W_LevelSelector.W_LevelSelector_C" (Game|GetPlayerController 0)))
      (bind _output_get_2 (Variables|Default|SetCurrentWidget _returnvalue_2))
      (UserInterface|Viewport|AddtoViewport _output_get_2 0))
    (:EGameplayWidget
      (Viewport|RemoveAllWidgets)
      (bind _returnvalue_3 (UserInterface|CreateWidget "/Game/Widgets/PlayerHUD.PlayerHUD_C" (Game|GetPlayerController 0)))
      (bind _output_get_3 (Variables|Default|SetCurrentWidget _returnvalue_3))
      (UserInterface|Viewport|AddtoViewport _output_get_3 0))
    (:ELoadingScreenWidget
      (Viewport|RemoveAllWidgets)
      (bind _returnvalue_4 (UserInterface|CreateWidget "/Game/Widgets/W_Loading.W_Loading_C" (Game|GetPlayerController 0)))
      (bind _output_get_4 (Variables|Default|SetCurrentWidget _returnvalue_4))
      (UserInterface|Viewport|AddtoViewport _output_get_4 0))
    (:EPauseMenuWidget
      (Viewport|RemoveAllWidgets)
      (bind _returnvalue_5 (UserInterface|CreateWidget "/Game/Widgets/W_PauseMenu.W_PauseMenu_C" (Game|GetPlayerController 0)))
      (bind _output_get_5 (Variables|Default|SetCurrentWidget _returnvalue_5))
      (UserInterface|Viewport|AddtoViewport _output_get_5 0))))