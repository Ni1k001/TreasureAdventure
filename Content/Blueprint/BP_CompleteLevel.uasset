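; Level completion trigger actor that unlocks the next level when something begins overlapping it.
; On the first overlap it finds the current level name among the LevelAvailability keys in TAGameInstance, marks the following key available and saves.
; It then fades camera and audio out and opens the level selector.
; When no following key exists, it neither saves nor leaves the level.
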(event Collision|EventActorBeginOverlap
  (params (OtherActor :type Actor%20Object%20Reference))
  (Utilities|FlowControl|DoOnce false
    (:Completed
      (bind _astagame_instance (Utilities|Casting|CastToTAGameInstance (Game|GetGameInstance)))
      (bind _returnvalue (Game|GetCurrentLevelName true))
      (bind _keys (Utilities|Map|Keys (Variables|/Script/TreasureAdventure.TAGameInstance|GetLevelAvailability _astagame_instance)))
      (if (Utilities|Array|IsValidIndex _keys (+ (Utilities|Array|FindItem _keys _returnvalue) 1))
        (Utilities|Map|Add (Variables|/Script/TreasureAdventure.TAGameInstance|GetLevelAvailability _astagame_instance) (Utilities|Array|Get(acopy) _keys (+ (Utilities|Array|FindItem _keys _returnvalue) 1)) true)
        (Class|TAGameInstance|SaveData _astagame_instance)
        (CameraFades|StartCameraFade :self (Game|GetPlayerCameraManager 0) :ToAlpha 1.0 :Duration 2.0 :bShouldFadeAudio true :bHoldWhenFinished true)
        (Utilities|FlowControl|Delay 2.0)
        (Game|OpenLevel(byName) "L_LevelSelector")))))

(fn ConstructionScript)