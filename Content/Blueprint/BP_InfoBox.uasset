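; BP_InfoBox is a one-shot trigger that shows the player an InfoBox widget with text matched to their input device.
; On player overlap it creates the widget, sets game-and-UI input, applies the pause setting and disables pawn input.
; While overlapped, Tick picks keyboard/mouse, PS4 or XO text from controller and game-instance state.
; Once the widget leaves the viewport it destroys its collision, and end overlap destroys the actor.
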(event Collision|EventActorBeginOverlap
  (params (OtherActor :type Actor%20Object%20Reference))
  (bind _returnvalue (Game|GetPlayerController 0))
  (if (== OtherActor (Game|GetPlayerCharacter 0))
    (Utilities|FlowControl|DoOnce false
      (:Completed
        (bind _returnvalue_2 (UserInterface|CreateWidget "/Game/Widgets/InfoBox.InfoBox_C" _returnvalue))
        (Input|SetInputModeGameandUI _returnvalue _returnvalue_2 "DoNotLock" true)
        (UserInterface|Viewport|AddtoViewport _returnvalue_2 0)
        (Game|SetGamePaused (Variables|Default|GetPause))
        (Input|DisableInput (Game|Player|GetPlayerPawn 0) _returnvalue)))))

(event Collision|EventActorEndOverlap
  (params (OtherActor :type Actor%20Object%20Reference))
  (Actor|DestroyActor))

(event EventTick
  (params (DeltaSeconds :type Float%20%28single-precision%29))
  (bind _returnvalue (Game|GetGameInstance))
  (bind (_asgame_instance_bp _bsuccess) (Utilities|Casting|CastToGameInstance_BP _returnvalue))
  (if (Collision|IsOverlappingActor (Game|GetPlayerCharacter 0) :!class /Script/Engine.Actor)
    (if (Variables|/Script/TreasureAdventure.TAPlayerController|GetbIsUsingGamepad (.AsPlayer%20Controller%20BP (Utilities|Casting|CastToPlayerController_BP (Game|GetPlayerController 0))))
      (if _bsuccess
        (if (Variables|/Script/TreasureAdventure.TAGameInstance|GetbControllerType _asgame_instance_bp)
          (Variables|/Game/Widgets/InfoBox.InfoBox_C|SetText (stale Collision|EventActorBeginOverlap _returnvalue_2) (Variables|Default|GetTextPS4))
          (else
            (Variables|/Game/Widgets/InfoBox.InfoBox_C|SetText (stale Collision|EventActorBeginOverlap _returnvalue_2) (Variables|Default|GetTextXO))))
        (if (not (UserInterface|Viewport|IsinViewport (stale Collision|EventActorBeginOverlap _returnvalue_2))) :!label _label
          (Components|DestroyComponent (Variables|Default|GetCollisionComponent))))
      (else
        (Variables|/Game/Widgets/InfoBox.InfoBox_C|SetText (stale Collision|EventActorBeginOverlap _returnvalue_2) (Variables|Default|GetTextMKb))
        (goto _label)))))

(fn ConstructionScript)